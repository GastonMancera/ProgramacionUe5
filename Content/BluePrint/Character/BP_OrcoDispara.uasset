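; Shooting orc character that moves continuously and can fire arrows.
; Tick adds VelOrco as a local offset without sweep, so movement is per frame and not scaled by delta time.
; SpawnFlecha spawns BP_Disparo at the orc's location, passing it the arrow speed and Multiplicador.
; Setters expose orc and arrow speeds; nothing in this Blueprint calls them or triggers firing.
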(event `self.ReceiveTick`
  (params (DeltaSeconds :type "Float (single-precision)"))
  (`self.K2_AddActorLocalOffset` (`self.VelOrco`)))

(fn `SetVelFlecha`
  (params (VelFlecha :type "Vector Structure"))
  (set `self.Velocidad Flecha` VelFlecha))

(fn `SetVelOrco`
  (params (Vel :type "Vector Structure"))
  (set `self.VelOrco` Vel))

(fn `SpawnFlecha`
  (`|SpawnActorFromClass` "/Game/BluePrint/Weapon/BP_Disparo.BP_Disparo_C" (`KismetMathLibrary.MakeTransform` (`self.K2_GetActorLocation`)) "Undefined" "MultiplyWithRoot" null (`self.Velocidad Flecha`) (`self.Multiplicador`) null))

(fn `UserConstructionScript`)